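; Player controller for the stealth game that manages the HUD, death and end-of-game sequences.
; BeginPlay adds the HUD and creates a wind audio component, keeping references to both.
; OnDeath unpossesses, fades to black under a death screen, then asks BP_GameModeStealth to restart after a delay.
; EndOfGame unpossesses, fades quickly, stops the wind, and shows an end screen followed by credits with the mouse cursor enabled.
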(event Custom|OnDeath
  ;[1 1 1] OnDeath
  (Pawn|UnPossess)
  (Widget|RemovefromParent (Variables|Default|GetHeadsUpDisplay))
  (CameraFades|StartCameraFade (Variables|Default|GetPlayerCameraManager) 0.0 1.0 3.0 "(R=0.000000,G=0.000000,B=0.000000,A=1.000000)" false true)
  (bind _returnvalue (UserInterface|CreateWidget "/Game/Death/WBP_DeathScreen.WBP_DeathScreen_C" self))
  (UserInterface|Viewport|AddtoViewport _returnvalue 0)
  (Utilities|FlowControl|Delay 3.0)
  (Widget|RemovefromParent _returnvalue)
  (bind _asbp_game_mode_stealth (Utilities|Casting|CastToBP_GameModeStealth (Game|GetGameMode)))
  (Class|GameMode|RestartGame _asbp_game_mode_stealth))

(event Custom|EndOfGame
  ;[1 1 1] EndGame
  (Pawn|UnPossess)
  (Widget|RemovefromParent (Variables|Default|GetHeadsUpDisplay))
  (CameraFades|StartCameraFade (Variables|Default|GetPlayerCameraManager) 0.0 1.0 0.1 "(R=0.000000,G=0.000000,B=0.000000,A=1.000000)" false true)
  (Audio|Components|Audio|Stop (Variables|Default|GetWindSoundRef))
  (bind _returnvalue (UserInterface|CreateWidget "/Game/EndOfGame/WBP_EndGame.WBP_EndGame_C" self))
  (UserInterface|Viewport|AddtoViewport _returnvalue 0)
  (Utilities|FlowControl|Delay 5.0)
  (Widget|RemovefromParent _returnvalue)
  (bind _returnvalue_2 (UserInterface|CreateWidget "/Game/Menus/MainMenu/WBP_Credits.WBP_Credits_C" self))
  (UserInterface|Viewport|AddtoViewport _returnvalue_2 0)
  (Variables|Default|SetbShowMouseCursor true)
  (bind _asbp_stealth_controller (Utilities|Casting|CastToBP_StealthController (Game|GetPlayerController 0)))
  (Input|SetInputModeGameandUI _asbp_stealth_controller _returnvalue_2 "DoNotLock" false))

(event EventBeginPlay
  ;[1 1 1] HUD on Beginplay
  (bind _returnvalue (UserInterface|CreateWidget "/Game/HUD/WBP_HeadsUpDisplay.WBP_HeadsUpDisplay_C"))
  (bind _output_get (Variables|Default|SetHeadsUpDisplay _returnvalue))
  (UserInterface|Viewport|AddtoViewport _output_get 0)
  ;[1 1 1] Play wind from start of game
  (bind _returnvalue_2 (AddComponent|AddAudioComponent false))
  (Variables|Default|SetWindSoundRef _returnvalue_2))

(fn ConstructionScript)