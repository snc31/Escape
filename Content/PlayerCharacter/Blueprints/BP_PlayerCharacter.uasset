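; Player character Blueprint for a stealth game, handling sprint, crouch toggle, pause menu, sword-hit damage and enemy takedowns.
; BeginPlay attaches a spawned dagger to a hand socket and caches the stealth controller's HUD.
; Takedown line-traces forward for an enemy, snaps behind it and plays a paired montage, briefly reparenting the spring arm to the spine.
; Damage plays a hit reaction and reduces health; death triggers ragdoll and notifies the controller.
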(event EventBeginPlay
  ;[1 1 1] BeginPlay
  (Utilities|FlowControl|Sequence
    (:then_0
      ;[1 1 1] Attach Dagger to players hand
      (bind _returnvalue (Game|SpawnActorfromClass "/Game/WeaponsUsed/Blueprints/BP_Dagger.BP_Dagger_C" (Transformation|GetSocketTransform (Variables|Character|GetMesh) "GuardEnemySwordSocket" "RTS_World") "Undefined" 0 0))
      (Transformation|AttachComponentToComponent _returnvalue (Variables|Character|GetMesh) "PlayerWeaponSocket" "SnapToTarget" "SnapToTarget" "SnapToTarget" true))
    (:then_1
      ;[1 1 1] Show "F to takedown" on display
      (Utilities|FlowControl|Delay 0.3)
      (Variables|Default|SetSelfReference self)
      (bind _asbp_stealth_controller (Utilities|Casting|CastToBP_StealthController (Game|GetPlayerController 0)))
      (Variables|Default|SetHeads%20Up%20Display (Variables|/Game/PlayerCharacter/Blueprints/BP_StealthController.BP_StealthController_C|GetHeadsUpDisplay _asbp_stealth_controller)))))

(event EventTakeDamage
  (params (Damage :type Float%20%28single-precision%29))
  ;[1 1 1] Take Damage
  (if (not (Audio|Components|Audio|IsPlaying (Variables|Character|GetMesh)))
    (Components|Animation|PlayAnimation (Variables|Character|GetMesh) "/Game/WARRIOR_SWORD_ANIMSET/Sword_Warrior/Animation_RM/Warrior_Sword_Hit_Front_Anim.Warrior_Sword_Hit_Front_Anim" false)
    (Utilities|FlowControl|Delay 0.1)
    (Components|Animation|SetAnimationMode (Variables|Character|GetMesh) "AnimationBlueprint")
    (Audio|PlaySoundatLocation "/Game/SFX_FPS_SWORD/Sword_Blood/AudioCue/Sword_Blood_21_Cue.Sword_Blood_21_Cue" (Transformation|GetActorLocation) "0, 0, 0" 1.0 1.0 0.0 0 0 0)
    (bind _output_get (Variables|Default|SetHealth (- (Variables|Default|GetHealth) Damage)))
    (if (<= _output_get 0.0)
      (Physics|SetSimulatePhysics (Variables|Character|GetMesh) true)
      (bind _asbp_stealth_controller (Utilities|Casting|CastToBP_StealthController (Pawn|GetController)))
      (Default|OnDeath _asbp_stealth_controller))))

(event Input|ActionEvents|InputActionPauseGame
  (params (Key :type Key%20Structure :default "None"))
  ;[1 1 1] Pause
  (:Pressed
    (CallFunction|PauseGame)))

(event Input|ActionEvents|InputActionSprint
  (params (Key :type Key%20Structure :default "None"))
  ;[1 1 1] Sprinting linked to InputMappings
  (:Pressed
    (CallFunction|StartSprint))
  (:Released
    (CallFunction|StopSprint)))

(event Input|ActionEvents|InputActionCrouch
  (params (Key :type Key%20Structure :default "None"))
  ;[1 1 1] Crouch
  (:Pressed
    (CallFunction|PlayerCrouch)))

(event Input|ActionEvents|InputActionTakedown
  (params (Key :type Key%20Structure :default "None"))
  ;[1 1 1] TakeDown
  (:Pressed
    (CallFunction|Takedown)
    (Utilities|FlowControl|Delay 0.01)
    (Pawn|Components|CharacterMovement|SetMovementMode (Variables|Character|GetCharacterMovement) "MOVE_Walking" 0)
    (Transformation|AttachComponentToComponent (Variables|Default|GetSpringArm) (Variables|Character|GetMesh) "head" "SnapToTarget" "SnapToTarget" "SnapToTarget" true)))

(fn ConstructionScript)

(fn StartSprint
  (Variables|/Script/Engine.CharacterMovementComponent|SetMaxWalkSpeed (Variables|Character|GetCharacterMovement) (Variables|Default|GetSprintSpeed))
  (Variables|Default|SetIsRun? true)
  (if (AI|Components|NavMovement|IsCrouching (Variables|Character|GetCharacterMovement))
    (Character|UnCrouch)
    (Variables|Default|SetIsCrouch? false)))

(fn StopSprint
  (Variables|/Script/Engine.CharacterMovementComponent|SetMaxWalkSpeed (Variables|Character|GetCharacterMovement) (Variables|Default|GetWalkSpeed))
  (Variables|Default|SetIsRun? false))

(fn PlayerCrouch
  (if (AI|Components|NavMovement|IsCrouching (Variables|Character|GetCharacterMovement))
    (Character|UnCrouch)
    (Variables|Default|SetIsCrouch? false)
    (else
      (Character|Crouch)
      (Variables|Default|SetIsCrouch? true))))

(fn PauseGame
  (bind _returnvalue (Game|GetPlayerController 0))
  ;[1 1 1] Pause and UnPause
  (Utilities|IsValid (Variables|Default|GetPauseMenuReference)
    (:Is%20Valid
      _)
    (:Is%20Not%20Valid
      (bind _returnvalue_2 (UserInterface|CreateWidget "/Game/Menus/PauseMenu/WBP_PauseMenu.WBP_PauseMenu_C"))
      (Variables|Default|SetPauseMenuReference _returnvalue_2)))
  (if (Game|IsGamePaused)
    (Widget|RemovefromParent (Variables|Default|GetPauseMenuReference))
    (Game|SetGamePaused false)
    (Variables|/Script/Engine.PlayerController|SetbShowMouseCursor _returnvalue false)
    (Input|SetInputModeGameOnly _returnvalue)
    (else
      (UserInterface|Viewport|AddtoViewport (Variables|Default|GetPauseMenuReference) 0)
      (Game|SetGamePaused true)
      (Variables|/Script/Engine.PlayerController|SetbShowMouseCursor _returnvalue true)
      (Input|SetInputModeGameandUI _returnvalue (Variables|Default|GetPauseMenuReference) "DoNotLock" false))))

(fn IsTakingDown?
  (return false))

(fn Takedown
  (bind _returnvalue (Transformation|GetActorLocation))
  (if (Variables|Default|GetCanTakedown?)
    (if (AI|Components|NavMovement|IsCrouching (Variables|Character|GetCharacterMovement))
      (Character|UnCrouch)
      (Variables|Default|SetIsCrouch? false)
      (else
        (bind (_outhit _returnvalue_2) (Collision|LineTraceByChannel _returnvalue (+ _returnvalue (* (Transformation|GetActorForwardVector) 5e+02)) "TraceTypeQuery1" false 0 "None"))
        (if _returnvalue_2
          (bind _asbp_enemy (Utilities|Casting|CastToBP_Enemy (.HitActor (Collision|BreakHitResult _outhit))))
          (Variables|Default|SetAs%20BP%20Enemy _asbp_enemy)
          (Transformation|AttachComponentToComponent (Variables|Default|GetSpringArm) (Variables|Character|GetMesh) "spine_02" "SnapToTarget" "SnapToTarget" "SnapToTarget" true)
          (Pawn|Components|CharacterMovement|DisableMovement (Variables|Character|GetCharacterMovement))
          (Variables|Default|SetCanTakedown? false)
          (Transformation|SetActorTransform (Math|Transform|MakeTransform (Math|Vector|MakeVector (.x (+ (* (Transformation|GetActorForwardVector (Variables|Default|GetAs%20BP%20Enemy)) -115.0) (.location (Transformation|GetActorTransform (Variables|Default|GetAs%20BP%20Enemy))))) (.y (+ (* (Transformation|GetActorForwardVector (Variables|Default|GetAs%20BP%20Enemy)) -115.0) (.location (Transformation|GetActorTransform (Variables|Default|GetAs%20BP%20Enemy))))) (.z (+ (* (Transformation|GetActorForwardVector (Variables|Default|GetAs%20BP%20Enemy)) -115.0) (.location (Transformation|GetActorTransform (Variables|Default|GetAs%20BP%20Enemy)))))) (.rotation (Transformation|GetActorTransform (Variables|Default|GetAs%20BP%20Enemy))) "1,1,1"))
          (bind _returnvalue_3 (Animation|PlayAnimMontage "/Game/StealthTakedownAnimationsUsed/Paired_Knife_Stealth_ClavicleStabDown_Att_Montage.Paired_Knife_Stealth_ClavicleStabDown_Att_Montage" 1.0 "None"))
          (Default|Takedown (Variables|Default|GetAs%20BP%20Enemy)))))))

(fn IsTakedowninProgress
  (return true))