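; Parent enemy Blueprint that lets the player perform a stealth knife takedown on it.
; Entering or leaving its TakedownArea toggles CanTakedown on the overlapping BP_PlayerCharacter.
; The Takedown event disables movement and collision, plays the paired victim montage, waits for its returned length, then destroys the actor.
; IsTakedownInProgress simply returns the CanBeTakenDown variable, which this graph never sets.
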(event OnComponentBeginOverlap(TakedownArea)
  (params (OverlappedComponent :type Primitive%20Component%20Object%20Reference) (OtherActor :type Actor%20Object%20Reference) (OtherComp :type Primitive%20Component%20Object%20Reference) (OtherBodyIndex :type Integer) (bFromSweep :type Boolean) (SweepResult :type Hit%20Result%20Structure%20%28by%20ref%29))
  ;[1 1 1] Receive Takedown from player
  (bind _asbp_player_character (Utilities|Casting|CastToBP_PlayerCharacter OtherActor))
  (Variables|/Game/PlayerCharacter/Blueprints/BP_PlayerCharacter.BP_PlayerCharacter_C|SetCanTakedown? _asbp_player_character true))

(event OnComponentEndOverlap(TakedownArea)
  (params (OverlappedComponent :type Primitive%20Component%20Object%20Reference) (OtherActor :type Actor%20Object%20Reference) (OtherComp :type Primitive%20Component%20Object%20Reference) (OtherBodyIndex :type Integer))
  ;[1 1 1] Receive Takedown from player
  (bind _asbp_player_character (Utilities|Casting|CastToBP_PlayerCharacter OtherActor))
  (Variables|/Game/PlayerCharacter/Blueprints/BP_PlayerCharacter.BP_PlayerCharacter_C|SetCanTakedown? _asbp_player_character false))

(event Custom|Takedown
  ;[1 1 1] Receive Takedown from player
  (Pawn|Components|CharacterMovement|DisableMovement (Variables|Character|GetCharacterMovement self))
  (Collision|SetActorEnableCollision self false)
  (bind _returnvalue (Animation|PlayAnimMontage "/Game/StealthTakedownAnimationsUsed/Paired_Knife_Stealth_ClavicleStabDown_Vic_Montage.Paired_Knife_Stealth_ClavicleStabDown_Vic_Montage" 1.0 "None"))
  (Utilities|FlowControl|Delay _returnvalue)
  (Actor|DestroyActor))

(event EventBeginPlay)

(event Collision|EventActorBeginOverlap
  (params (OtherActor :type Actor%20Object%20Reference)))

(event EventTick
  (params (DeltaSeconds :type Float%20%28single-precision%29)))

(fn ConstructionScript)

(fn IsTakedowninProgress
  (return (Variables|Default|GetCanBeTakenDown)))