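; AI controller for guard enemies that runs the guard behaviour tree and forwards attack calls to its controlled guard pawn.
; Perception updates for the player are routed by sense class to HandleSense, which writes the investigation flag and target keys to the Blackboard.
; Sight sets the player as target actor and raises walk speed, while losing sight or hearing stores the stimulus location to investigate.
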(event OnTargetPerceptionUpdated(AIPerception)
  (params (Actor :type Actor%20Object%20Reference) (Stimulus :type AI%20Stimulus%20Structure))
  ;[1 1 1] GuardPerception
  (Variables|Default|SetActor Actor)
  (Variables|Default|SetStimulus Stimulus)
  (bind _asbp_player_character (Utilities|Casting|CastToBP_PlayerCharacter (Game|GetPlayerCharacter 0)))
  (if (== _asbp_player_character (Variables|Default|GetActor))
    (bind _returnvalue (Class|AIPerceptionSystem|GetSenseClassforStimulus (Variables|Default|GetStimulus)))
    (CallFunction|HandleSense (Utilities|GetClassDisplayName _returnvalue) (Variables|Default|GetStimulus) (Variables|Default|GetActor))))

(event Custom|Pawn_Attack
  ;[1 1 1] Guard Attack
  (Default|Attack (Variables|Default|GetAs%20BP%20Guard%20Enemy)))

(event EventBeginPlay
  ;[1 1 1] Store cast in memory at begin play
  (bind _asbp_guard_enemy (Utilities|Casting|CastToBP_GuardEnemy (Pawn|GetControlledPawn)))
  (Variables|Default|SetAs%20BP%20Guard%20Enemy _asbp_guard_enemy)
  ;[1 1 1] Run Guard Behaviour Tree
  (AI|RunBehaviorTree "/Game/AI/EnemyAI/Guard/BehaviourTrees/BT_GuardBehaviour.BT_GuardBehaviour"))

(event EventTick
  (params (DeltaSeconds :type Float%20%28single-precision%29)))

(fn ConstructionScript)

(fn HandleSense
  (params (Selection :type String) (Stimulus :type AI%20Stimulus%20Structure) (SensedActor :type Actor%20Object%20Reference))
  (switch string Selection
    (:AiSense_Sight
      ;[1 1 1] AI Sees
      (AI|Components|Blackboard|SetValueasBool (Variables|Default|GetBlackboard) (Utilities|Name|MakeLiteralName "IsInvestigating?") (.bsuccessfullysensed Stimulus))
      (if (.bsuccessfullysensed Stimulus)
        (if (== SensedActor (Game|GetPlayerCharacter 0))
          (AI|Components|Blackboard|SetValueasObject (Variables|Default|GetBlackboard) (Utilities|Name|MakeLiteralName "TargetLocationActor") SensedActor)
          (bind _ascharacter (Utilities|Casting|CastToCharacter (Pawn|GetControlledPawn)))
          (Variables|/Script/Engine.CharacterMovementComponent|SetMaxWalkSpeed (Variables|/Script/Engine.Character|GetCharacterMovement _ascharacter) 6e+02)
          (else
            (AI|Components|Blackboard|SetValueasBool (Variables|Default|GetBlackboard) (Utilities|Name|MakeLiteralName "IsInvestigating?") false)))
        (else
          (AI|Components|Blackboard|SetValueasVector (Variables|Default|GetBlackboard) (Utilities|Name|MakeLiteralName "TargetLocationVector") (.stimuluslocation Stimulus))
          (AI|Components|Blackboard|SetValueasObject (Variables|Default|GetBlackboard) (Utilities|Name|MakeLiteralName "TargetLocationActor") 0))))
    (:AISense_Hearing
      ;[1 1 1] AI Hearing
      (AI|Components|Blackboard|SetValueasBool (Variables|Default|GetBlackboard) (Utilities|Name|MakeLiteralName "IsInvestigating?") (.bsuccessfullysensed Stimulus))
      (AI|Components|Blackboard|SetValueasVector (Variables|Default|GetBlackboard) (Utilities|Name|MakeLiteralName "TargetLocationVector") (.stimuluslocation Stimulus)))))